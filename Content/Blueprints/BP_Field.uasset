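; BP_Field is a Paper2D field actor built from repeated stage segments with two box lanes spanning its length.
; The construction script adds one field sprite component per stage, spaced along X by stage size.
; It then stretches Lane1 and Lane2 along X to cover all stages and centers them on the row, keeping their Y and Z values.
; The event graph holds no active logic.
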(event EventBeginPlay)

(event Collision|EventActorBeginOverlap
  (params (OtherActor :type Actor%20Object%20Reference)))

(event EventTick
  (params (DeltaSeconds :type Float%20%28single-precision%29)))

(fn ConstructionScript
  (for _index (range 0 (- (Variables|Default|GetStageQuantity) 1))
    (bind _returnvalue (AddComponent|AddPaperSpriteComponent false (Math|Transform|MakeTransform (Math|Vector|MakeVector (Math|Conversions|ToFloat(Integer) (* _index (Variables|Default|GetStageSize))) 0.0 0.0) "0, 0, 0" "1.000000,1.000000,1.000000")))
    (Rendering|Components|Sprite|SetSprite _returnvalue "/Game/Assets/Background/S_Field.S_Field"))
  (CallFunction|UpdateBoxExtend (Variables|Default|GetLane1))
  (CallFunction|UpdateBoxExtend (Variables|Default|GetLane2))
  (CallFunction|UpdateBoxLocattion (Variables|Default|GetLane1))
  (CallFunction|UpdateBoxLocattion (Variables|Default|GetLane2)))

(fn UpdateBoxExtend
  (params (Lane :type Box%20Component%20Object%20Reference))
  (bind _boxextent (Variables|/Script/Engine.BoxComponent|GetBoxExtent Lane))
  (Components|Box|SetBoxExtent Lane (Math|Vector|MakeVector (Math|Conversions|ToFloat(Integer) (* (/ (Variables|Default|GetStageSize) 2) (Variables|Default|GetStageQuantity))) (.y _boxextent) (.z _boxextent)) true))

(fn UpdateBoxLocattion
  (params (Lane :type Scene%20Component%20Object%20Reference))
  (bind _relativelocation (Variables|/Script/Engine.SceneComponent|GetRelativeLocation Lane))
  (Transformation|SetRelativeLocation Lane (Math|Vector|MakeVector (Math|Conversions|ToFloat(Integer) (- (/ (* (Variables|Default|GetStageSize) (Variables|Default|GetStageQuantity)) 2) (/ (Variables|Default|GetStageSize) 2))) (.y _relativelocation) (.z _relativelocation)) false false))