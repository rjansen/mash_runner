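; AI controller that drives a BP_Runner by simulating alternating left and right power inputs.
; On possess it caches and prints the runner, while BeginPlay starts a one-shot timer with a random delay between configurable bounds.
; SimulateInput flip-flops between AIPowerLeft and AIPowerRight on the runner, then re-arms the timer for irregularly paced input.
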(event Custom|SimulateInput
  (Utilities|FlowControl|FlipFlop
    (:A
      (Default|AIPowerLeft (Variables|Default|GetRunner)))
    (:B
      (Default|AIPowerRight (Variables|Default|GetRunner))))
  (CallFunction|SimulateInputwithDelay))

(event EventBeginPlay
  (CallFunction|SimulateInputwithDelay))

(event EventPossess
  (params (PossessedPawn :type Pawn%20Object%20Reference))
  (bind _asbp_runner (Utilities|Casting|CastToBP_Runner PossessedPawn))
  (bind _output_get (Variables|Default|SetRunner _asbp_runner))
  (Development|PrintString (Utilities|GetDisplayName _output_get)))

(fn ConstructionScript)

(fn SimulateInputwithDelay
  (Utilities|Time|SetTimerbyEvent (EventDispatchers|CreateEvent :!event Custom|SimulateInput) (Math|Random|RandomFloatinRange (Variables|Default|GetMinPlayDelay) (Variables|Default|GetMaxPlayDelay))))